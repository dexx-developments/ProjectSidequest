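; City street generator actor that lines both sides of a Road spline with randomly chosen house actors.
; UpdateRoad, repeatable on a looping timer, destroys old houses, then spawns and attaches seeded-random variants at even spacing, offset perpendicular to the spline.
; Optional line traces snap houses down onto terrain or landscape.
; Optionally paints the road onto a selected landscape layer through EditorApplySpline.
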(event Collision|EventActorBeginOverlap
  (params (OtherActor :type Actor%20Object%20Reference)))

(event EventTick
  (params (DeltaSeconds :type Float%20%28single-precision%29)))

(fn ConstructionScript)

(fn GetHouseTransform
  (params (SplineIndex :type Integer))
  (bind _road (Variables|Default|GetRoad))
  (bind _space (Variables|HousePlacement|GetSpace))
  (bind _returnvalue (* SplineIndex _space))
  (bind _returnvalue_2 (Spline|GetTransformatDistanceAlongSpline _road _returnvalue "World" false))
  (bind (_location _rotation) (Math|Transform|BreakTransform _returnvalue_2))
  (return (Math|Transform|MakeTransform (+ (* (Math|Vector|RotateVectorAroundAxis (Spline|GetDirectionatDistanceAlongSpline _road _returnvalue "World") 9e+01 "0.000000, 0,1.000000") (Variables|HousePlacement|GetBuildDistanceAwayFromRoad)) _location) (Math|Rotator|MakeRotator 0.0 0.0 (+ (.Yaw (Math|Rotator|BreakRotator _rotation)) (Variables|HousePlacement|GetMeshRotate))))))

(fn SnaptoTerrain
  (params (SpawnedActor :type Actor%20Object%20Reference%20%28by%20ref%29))
  (bind _rootcomponent (Variables|/Script/Engine.Actor|GetRootComponent SpawnedActor))
  (bind _returnvalue (Transformation|GetWorldLocation _rootcomponent))
  (bind (_x _y _z) (Math|Vector|BreakVector _returnvalue))
  (bind (_x_2 _y_2 _z_2) (Math|Vector|BreakVector _returnvalue))
  (if (Variables|HousePlacement|GetStickToTerrain)
    (if (Variables|HousePlacement|GetLandscapeStickOnly)
      (LocalVariables|SetTraceType "TraceTypeQuery3")
      (else
        (LocalVariables|SetTraceType "TraceTypeQuery1")))
    (bind _outhit (Collision|LineTraceByChannel (Math|Vector|MakeVector _x_2 _y_2 (+ _z_2 (LocalVariables|GetBottomSensitivity))) (Math|Vector|MakeVector _x _y (+ _z -2e+04)) (LocalVariables|GetTraceType) false 0 "None"))
    (Transformation|AddRelativeLocation (Variables|/Script/Engine.Actor|GetRootComponent SpawnedActor) (Math|Vector|MakeVector 0.0 0.0 (- (- (.Z (Math|Vector|BreakVector (.Location (Collision|BreakHitResult _outhit)))) (Variables|HousePlacement|GetExtraTerrainSink)) _z_2)) false false)))

(fn SpawnActor
  (params (transformToSpawnAt :type Transform))
  (switch int (Math|Random|RandomIntegerinRangefromStream 0 (- (Variables|HousePlacement|GetHouse%20Variations) 1) (Variables|HousePlacement|GetRandomStream))
    (:0
      (bind _spawnedactor (CallFunction|SpawnHouse transformToSpawnAt (Variables|HouseVariations|GetHouse1%20%28Don't%20change,%20Open%20FSCG_House1%20to%20customize%29)))
      (return _spawnedactor))
    (:1
      (bind _spawnedactor_2 (CallFunction|SpawnHouse transformToSpawnAt (Variables|HouseVariations|GetHouse2%20%28Don't%20change,%20Open%20FSCG_House1%20to%20customize%29)))
      (return _spawnedactor_2))
    (:2
      (bind _spawnedactor_3 (CallFunction|SpawnHouse transformToSpawnAt (Variables|HouseVariations|GetHouse3%20%28Don't%20change,%20Open%20FSCG_House3%20to%20customize%29)))
      (return _spawnedactor_3))
    (:3
      (bind _spawnedactor_4 (CallFunction|SpawnHouse transformToSpawnAt (Variables|HouseVariations|GetHouse4%20%28Don't%20change,%20Open%20FSCG_House4%20to%20customize%29)))
      (return _spawnedactor_4))
    (:4
      (bind _spawnedactor_5 (CallFunction|SpawnHouse transformToSpawnAt (Variables|HouseVariations|GetHouse5%20%28Don't%20change,%20Open%20FSCG_House5%20to%20customize%29)))
      (return _spawnedactor_5))
    (:5
      (bind _spawnedactor_6 (CallFunction|SpawnHouse transformToSpawnAt (Variables|HouseVariations|GetHouse6%20%28Don't%20change,%20Open%20FSCG_House6%20to%20customize%29)))
      (return _spawnedactor_6))
    (:6
      (bind _spawnedactor_7 (CallFunction|SpawnHouse transformToSpawnAt (Variables|HouseVariations|GetHouse7%20%28Don't%20change,%20Open%20FSCG_House7%20to%20customize%29)))
      (return _spawnedactor_7))
    (:7
      (bind _spawnedactor_8 (CallFunction|SpawnHouse transformToSpawnAt (Variables|HouseVariations|GetHouse8%20%28Don't%20change,%20Open%20FSCG_House8%20to%20customize%29)))
      (return _spawnedactor_8))
    (:8
      (bind _spawnedactor_9 (CallFunction|SpawnHouse transformToSpawnAt (Variables|HouseVariations|GetHouse9%20%28Don't%20change,%20Open%20FSCG_House9%20to%20customize%29)))
      (return _spawnedactor_9))
    (:9
      (bind _spawnedactor_10 (CallFunction|SpawnHouse transformToSpawnAt (Variables|HouseVariations|GetHouse10%20%28Don't%20change,%20Open%20FSCG_House10%20to%20customize%29)))
      (return _spawnedactor_10))))

(fn UpdateRoad
  (bind _road (Variables|Default|GetRoad))
  (bind _space (Variables|HousePlacement|GetSpace))
  (bind _returnvalue (Spline|GetSplineLength _road))
  (bind _returnvalue_2 (Math|Float|Division(WholeandRemainder) _returnvalue _space))
  (for _array_element (Variables|HouseVariations|GetHouses)
    (bind _asfcsg_house_1 (Utilities|Casting|CastToFCSG_House1 _array_element)
      (:then
        (Default|Destroy _asfcsg_house_1))
      (:CastFailed
        (bind _asfcsg_house_2 (Utilities|Casting|CastToFCSG_House2 _array_element)
          (:then
            (Default|Destroy _asfcsg_house_2))
          (:CastFailed
            (bind _asfcsg_house_3 (Utilities|Casting|CastToFCSG_House3 _array_element)
              (:then
                (Default|Destroy _asfcsg_house_3))
              (:CastFailed
                (bind _asfcsg_house_4 (Utilities|Casting|CastToFCSG_House4 _array_element)
                  (:then
                    (Default|Destroy _asfcsg_house_4))
                  (:CastFailed
                    (bind _asfcsg_house_5 (Utilities|Casting|CastToFCSG_House5 _array_element)
                      (:then
                        (Default|Destroy _asfcsg_house_5))
                      (:CastFailed
                        (bind _asfcsg_house_6 (Utilities|Casting|CastToFCSG_House6 _array_element)
                          (:then
                            (Default|Destroy _asfcsg_house_6))
                          (:CastFailed
                            (bind _asfcsg_house_7 (Utilities|Casting|CastToFCSG_House7 _array_element)
                              (:then
                                (Default|Destroy _asfcsg_house_7))
                              (:CastFailed
                                (bind _asfcsg_house_8 (Utilities|Casting|CastToFCSG_House8 _array_element)
                                  (:then
                                    (Default|Destroy _asfcsg_house_8))
                                  (:CastFailed
                                    _))
                                (bind _asfcsg_house_9 (Utilities|Casting|CastToFCSG_House9 _array_element)
                                  (:then
                                    (Default|Destroy _asfcsg_house_9))
                                  (:CastFailed
                                    (bind _asfcsg_house_10 (Utilities|Casting|CastToFCSG_House10 _array_element))
                                    (Default|Destroy _asfcsg_house_10))))))))))))))))))
  (Utilities|Array|Clear (Variables|HouseVariations|GetHouses))
  (if (Variables|LandscapePainting|GetPaint%20Road%20Whille%20Moving)
    (LandscapePainting|PaintRoad))
  (if (< (Variables|HousePlacement|GetBuildDistanceAwayFromRoad) 0.0)
    (Variables|HousePlacement|SetBuildDistanceAwayFromRoad (* (Variables|HousePlacement|GetBuildDistanceAwayFromRoad) -1.0)))
  (if (Variables|HousePlacement|GetSpawnRightHouses)
    (for _index (range 0 _returnvalue_2)
      ;[1 1 1] Right Side Buildings
      (bind _housetrasform (CallFunction|GetHouseTransform _index))
      (bind _spawned_actor (CallFunction|SpawnActor _housetrasform))
      (CallFunction|SnaptoTerrain _spawned_actor)))
  (if (Variables|HousePlacement|GetSpawnLeftHouses)
    (Variables|HousePlacement|SetBuildDistanceAwayFromRoad (* -1.0 (Variables|HousePlacement|GetBuildDistanceAwayFromRoad)))
    ;[1 1 1] Left Side Buildings
    (for _index_2 (range 0 _returnvalue_2)
      (bind _housetrasform_2 (CallFunction|GetHouseTransform _index_2))
      (bind _spawned_actor_2 (CallFunction|SpawnActor _housetrasform_2))
      (CallFunction|SnaptoTerrain _spawned_actor_2))))

(fn SpawnHouse
  (params (SpawnTransform :type Transform%20%28by%20ref%29) (ClassToSpawn :type Actor%20Class%20Reference%20%28by%20ref%29))
  (bind _returnvalue (Game|SpawnActorfromClass ClassToSpawn SpawnTransform "Undefined" 0 0))
  (Transformation|AttachActorToActor _returnvalue self "None" "KeepWorld" "KeepWorld" "KeepWorld" false)
  (Utilities|Array|Add (Variables|HouseVariations|GetHouses) _returnvalue)
  (return _returnvalue))

(fn PaintRoad
  (bind _roadtexturewidth (Variables|LandscapePainting|GetRoadTextureWidth))
  (Landscape|Editor|EditorApplySpline (Variables|LandscapePainting|GetSelected%20Landscape%20%28Required%20for%20road%20painting%20to%20work%29) (Variables|Default|GetRoad) _roadtexturewidth _roadtexturewidth 2e+02 2e+02 0.0 0.0 20 false false (Variables|LandscapePainting|GetRoadPaintLayer)))

(fn StartUpdatingRoad
  (bind _returnvalue (Utilities|Time|SetTimerbyFunctionName 0 "UpdateRoad" (Variables|UpdateRoadAutomatically|GetRoadUpdateTime) true))
  (Variables|UpdateRoadAutomatically|SetUpdate%20Road%20Timer _returnvalue))

(fn StopUpdatingRoad
  (Utilities|Time|SetTimerbyFunctionName 0 "UpdateRoad" 0.0))