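; A test Blueprint that scatters rock meshes along a spline.
; The construction script divides spline length by a spacing value and adds a manually attached static mesh component at each step, using world-space spline locations.
; A random stream gives each rock repeatable pitch and non-uniform per-axis scale variation, then the rock mesh and material are assigned.
; The event graph holds only disabled stub events.
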(event EventBeginPlay)

(event Collision|EventActorBeginOverlap
  (params (OtherActor :type Actor%20Object%20Reference)))

(event EventTick
  (params (DeltaSeconds :type Float%20%28single-precision%29)))

(fn ConstructionScript
  (bind _randomrotation (Variables|Default|GetRandomRotation))
  (bind _randomstream (Variables|Default|GetRandomStream))
  (bind _randomscale (Variables|Default|GetRandomScale))
  (bind _returnvalue (Math|Random|RandomFloatinRangefromStream 0.8 _randomscale _randomstream))
  ;[1 1 1] Loop and Set Mesh
  (for _index (range 0 (.ReturnValue (Math|Float|Division(WholeandRemainder) (Spline|GetSplineLength (Variables|Default|GetSpline)) (Variables|Default|GetSpacing))))
    (bind _returnvalue_2 (AddComponent|AddStaticMeshComponent true (Math|Transform|MakeTransform (Spline|GetLocationatDistanceAlongSpline (Variables|Default|GetSpline) (* _index (Variables|Default|GetSpacing)) "World") (Math|Rotator|MakeRotator 0.0 (Math|Random|RandomFloatinRangefromStream (* _randomrotation -1.0) _randomrotation (Variables|Default|GetRandomStream)) 0.0) (Math|Vector|MakeVector _returnvalue _returnvalue _returnvalue))))
    (Components|StaticMesh|SetStaticMesh _returnvalue_2 "/Game/StarterContent/Props/SM_Rock.SM_Rock")
    (Rendering|Material|SetMaterial _returnvalue_2 0 "/Game/StarterContent/Props/Materials/M_Rock.M_Rock")))